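; Spline trail actor that moves a static mesh along a spline while feeding its transform to a Niagara effect.
; On BeginPlay a timeline maps its track to spline distance, setting the mesh's world location and rotation, with playback speed set by NewRate.
; Tick passes the mesh's location and forward-vector quaternion to Niagara as OriginLocation and OriginRotator.
; The construction script seeds both parameters from the actor's transform.
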(event EventBeginPlay
  (bind _spline (Variables|Default|GetSpline))
  (bind _staticmesh (Variables|Default|GetStaticMesh))
  (bind _newtrack_0 (Timeline|Timeline_0 PlayFromStart)
    (:Update
      (Transformation|SetWorldLocation _staticmesh (Spline|GetLocationatDistanceAlongSpline _spline (* _newtrack_0 (Spline|GetSplineLength (Variables|Default|GetSpline))) "World") false false)
      (Components|Timeline|SetPlayRate (Variables|Default|GetTimeline_0) (Variables|Default|GetNewRate))
      (Transformation|SetWorldRotation _staticmesh (Math|Rotator|MakeRotator (.Roll (Math|Rotator|BreakRotator (Spline|GetRotationatDistanceAlongSpline _spline (* _newtrack_0 (Spline|GetSplineLength (Variables|Default|GetSpline))) "World"))) (.Pitch (Math|Rotator|BreakRotator (Spline|GetRotationatDistanceAlongSpline _spline (* _newtrack_0 (Spline|GetSplineLength (Variables|Default|GetSpline))) "World"))) (.Yaw (Math|Rotator|BreakRotator (Spline|GetRotationatDistanceAlongSpline _spline (* _newtrack_0 (Spline|GetSplineLength (Variables|Default|GetSpline))) "World")))) false false))))

(event EventTick
  (params (DeltaSeconds :type Float%20%28single-precision%29))
  (bind _staticmesh (Variables|Default|GetStaticMesh))
  (Class|NiagaraComponent|SetNiagaraVariableVec3 (Variables|Default|GetNiagara) "OriginLocation" (Transformation|GetWorldLocation _staticmesh))
  (Class|NiagaraComponent|SetNiagaraVariableQuat (Variables|Default|GetNiagara) "OriginRotator" (Math|Conversions|ToQuaternion(Rotator) (Math|Vector|GetForwardVector (Transformation|GetWorldRotation _staticmesh)))))

(fn ConstructionScript
  (Class|NiagaraComponent|SetNiagaraVariableVec3 (Variables|Default|GetNiagara) "OriginLocation" (Transformation|GetActorLocation))
  (Class|NiagaraComponent|SetNiagaraVariableQuat (Variables|Default|GetNiagara) "OriginRotator" (Math|Conversions|ToQuaternion(Rotator) (Math|Vector|GetForwardVector (Transformation|GetActorRotation)))))