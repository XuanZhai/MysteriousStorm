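; Rocket projectile actor that spawns sparks on launch and destroys itself after a short delay.
; On Sphere hit it adds Niagara effects, pushes physics-simulating components with directional, upward and radial impulses, and places a randomized, fading bullet-hole decal.
; It then removes the Sphere while the actor awaits timed destruction.
; Impulse direction derives from Startposition, whose assignment is disconnected and never runs.
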(event OnComponentHit(Sphere)
  (params (HitComponent :type Primitive%20Component%20Object%20Reference) (OtherActor :type Actor%20Object%20Reference) (OtherComp :type Primitive%20Component%20Object%20Reference) (NormalImpulse :type Vector :default "0, 0, 0") (Hit :type Hit%20Result%20Structure%20%28by%20ref%29))
  ;[1 1 1] Hit component to variable
  (Variables|Default|SetOther%20Comp OtherComp)
  ;[1 1 1] Hit result
  (Variables|Default|SetHit Hit)
  ;[1 1 1] Since "Sphere" is pending kill, check if it is valid.
  (Utilities|IsValid (Variables|Default|GetSphere)
    (:Is%20Valid
      ;[1 1 1] When hitting something, add niagara particles at current projectile location.
      (AddComponent|AddNiagaraComponent false (Math|Transform|MakeTransform "0, 0, 0" "0, 0, 0" "0.100000,1.000000,1"))
      ;[1 1 1] spawn niagara system at hit location
      (Niagara|SpawnSystematLocation "/Game/MechaDestroyer/FX/NS_Sparks.NS_Sparks" (.Location (Collision|BreakHitResult (Variables|Default|GetHit))))
      ;[1 1 1] Is other comp still valid?
      (Utilities|IsValid (Variables|Default|GetOther%20Comp)
        (:Is%20Valid
          ;[1 1 1] If hit other component was simulating physics then add impulse.
          (if (Physics|IsSimulatingPhysics (Variables|Default|GetOther%20Comp) "None")
            ;[1 1 1] Add impulse to direction the projectile was moving. Add z vector ad radial impulse.
            (Physics|AddImpulse (Variables|Default|GetOther%20Comp) (+ (* (Math|Vector|GetForwardVector (Math|Rotator|FindLookatRotation (Variables|Default|GetStartposition) (.Location (Collision|BreakHitResult (Variables|Default|GetHit))))) 4e+03) (* "0, 0,1.000000" 1e+03)) "None" true)
            (Physics|AddRadialImpulse (Variables|Default|GetOther%20Comp) (Math|Vector|MakeVector (.X (Math|Vector|BreakVector (Transformation|GetWorldLocation (Variables|Default|GetOther%20Comp)))) (.Y (Math|Vector|BreakVector (Transformation|GetWorldLocation (Variables|Default|GetOther%20Comp)))) (- (.Z (Math|Vector|BreakVector (Transformation|GetWorldLocation (Variables|Default|GetOther%20Comp)))) -2e+02)) 5e+02 7.5e+03 "RIF_Linear" true))
          ;[1 1 1] Spawn decal and set decal fade out.
          (bind _returnvalue (Rendering|Decal|SpawnDecalatLocation (Utilities|Array|Get(acopy) (Utilities|Array|MakeArray "/Game/MechaDestroyer/MAT/INST/MI_Bullethole.MI_Bullethole" "/Game/MechaDestroyer/MAT/INST/MI_Bullethole_02.MI_Bullethole_02" "/Game/MechaDestroyer/MAT/INST/MI_Bullethole_03.MI_Bullethole_03" "/Game/MechaDestroyer/MAT/INST/MI_Bullethole_04.MI_Bullethole_04") (Math|Random|RandomIntegerinRange 0 3)) (* "100.000000,300.000000,300.000000" (Math|Random|RandomFloatinRange 0.8 1.2)) (.Location (Collision|BreakHitResult (Variables|Default|GetHit))) (Math|Rotator|MakeRotator (+ (.Roll (Math|Rotator|BreakRotator (Math|Conversions|RotationFromXVector (.Normal (Collision|BreakHitResult (Variables|Default|GetHit)))))) (Math|Random|RandomFloatinRange -1.8e+02 1.8e+02)) (.Pitch (Math|Rotator|BreakRotator (Math|Conversions|RotationFromXVector (.Normal (Collision|BreakHitResult (Variables|Default|GetHit)))))) (.Yaw (Math|Rotator|BreakRotator (Math|Conversions|RotationFromXVector (.Normal (Collision|BreakHitResult (Variables|Default|GetHit))))))) 0.0))
          (Rendering|Components|Decal|SetFadeOut _returnvalue 7.0 2.0 true)
          ;[1 1 1] If still valid, Remove sphere component.
          (Utilities|IsValid (Variables|Default|GetSphere)
            (:Is%20Valid
              (Components|DestroyComponent (Variables|Default|GetSphere)))))))))

(event EventBeginPlay
  ;[1 1 1] spawn emitter at spawn location.
  (Niagara|SpawnSystematLocation "/Game/MechaDestroyer/FX/NS_Sparks_Smaller.NS_Sparks_Smaller" (+ (Transformation|GetActorLocation) (* (Transformation|GetActorForwardVector) -1.5e+02)))
  ;[1 1 1] After spawning the projectile in 3 seconds destroy it if not already destroyed (if it did not hit anything).
  (Utilities|FlowControl|Delay 3.0)
  (Utilities|IsValid self
    (:Is%20Valid
      (Actor|DestroyActor))))

(fn ConstructionScript)