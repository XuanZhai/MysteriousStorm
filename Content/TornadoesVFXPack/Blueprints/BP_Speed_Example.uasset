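; BP_Speed_Example is an example actor for the tornado VFX pack that shows tornadoes spawned with different Speed values.
; On BeginPlay it spawns Light, Water and Bloody tornadoes in a row along X around its own location, overriding Speed on the outer two.
; A custom NewTornado event loops back after a delay, respawning the trio every few seconds with no cleanup in this graph.
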(event Custom|NewTornado
  (bind _returnvalue (Transformation|GetActorLocation))
  (bind _returnvalue_2 (Transformation|GetActorRotation))
  (Utilities|FlowControl|Sequence
    (:then_0
      (Game|SpawnActorfromClass "/Game/TornadoesVFXPack/Blueprints/BP_Light_Tornado.BP_Light_Tornado_C" (Math|Transform|MakeTransform (- _returnvalue "600.000000, 0, 0") _returnvalue_2 "1,1,1") "Undefined" 0 6.0 1.0 4e+01 false 4.0 0.0 0)
      (Game|SpawnActorfromClass "/Game/TornadoesVFXPack/Blueprints/BP_Water_Tornado.BP_Water_Tornado_C" (Math|Transform|MakeTransform _returnvalue _returnvalue_2 "1,1,1") "Undefined" 0 6.0 1.0 4e+01 false 4.0 1.0 0)
      (Game|SpawnActorfromClass "/Game/TornadoesVFXPack/Blueprints/BP_Bloody_Tornado.BP_Bloody_Tornado_C" (Math|Transform|MakeTransform (+ _returnvalue "600.000000, 0,0.000000") _returnvalue_2 "1,1,1") "Undefined" 0 6.0 1.0 4e+01 false 4.0 3.0 0))
    (:then_1
      (Utilities|FlowControl|Delay 7.0)
      (CallFunction|NewTornado))))

(event EventBeginPlay
  (bind _returnvalue (Transformation|GetActorLocation))
  (bind _returnvalue_2 (Transformation|GetActorRotation))
  (Utilities|FlowControl|Sequence
    (:then_0
      (Game|SpawnActorfromClass "/Game/TornadoesVFXPack/Blueprints/BP_Light_Tornado.BP_Light_Tornado_C" (Math|Transform|MakeTransform (- _returnvalue "600.000000, 0, 0") _returnvalue_2 "1,1,1") "Undefined" 0 6.0 1.0 4e+01 false 4.0 0.0 0)
      (Game|SpawnActorfromClass "/Game/TornadoesVFXPack/Blueprints/BP_Water_Tornado.BP_Water_Tornado_C" (Math|Transform|MakeTransform _returnvalue _returnvalue_2 "1,1,1") "Undefined" 0 6.0 1.0 4e+01 false 4.0 1.0 0)
      (Game|SpawnActorfromClass "/Game/TornadoesVFXPack/Blueprints/BP_Bloody_Tornado.BP_Bloody_Tornado_C" (Math|Transform|MakeTransform (+ _returnvalue "600.000000, 0,0.000000") _returnvalue_2 "1,1,1") "Undefined" 0 6.0 1.0 4e+01 false 4.0 3.0 0))
    (:then_1
      (Utilities|FlowControl|Delay 7.0)
      (CallFunction|NewTornado))))

(fn ConstructionScript)