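; BP_TestEnemyAbility is a test enemy ability that decides whether it can activate against the player.
; CheckPrecondition requires CheckPreconditionImplementation to pass, an interval time comparison to hold, and the owning MSEnemyCharacter to be within a fixed distance of the player.
; The player's position comes from the enemy controller's Blackboard key PlayerLocation.
; TryActivateAbility only returns that precondition result and performs no ability action.
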(fn CheckPrecondition
  (bind _ownerenemy (Variables|Default|GetOwnerEnemy))
  (bind _asmsenemy_character (Utilities|Casting|CastToMSEnemyCharacter _ownerenemy))
  (bind _returnvalue (Class|MSEnemyAbility|CheckPreconditionImplementation))
  (return (and _returnvalue (and (>= (Variables|Default|GetIntervalTime) (Variables|Default|GetIntervalTimer)) (< (Math|Vector|Distance(Vector) (Transformation|GetActorLocation _ownerenemy) (AI|Components|Blackboard|GetValueasVector (AI|GetBlackboard (Pawn|GetController _asmsenemy_character)) (Utilities|Name|MakeLiteralName "PlayerLocation"))) 5e+02)))))

(fn TryActivateAbility
  (bind _returnvalue (CallFunction|CheckPrecondition))
  (return _returnvalue))