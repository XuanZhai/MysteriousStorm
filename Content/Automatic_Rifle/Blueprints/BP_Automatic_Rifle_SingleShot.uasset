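; Automatic rifle actor that plays a single-shot effect whenever something enters or leaves its trigger box.
; BeginPlay attaches the core and cartridge case to rifle sockets and sets emissive and digital-plate material parameters.
; Each shot plays animation, sound and particles, with timed delays blinking the cartridge case and pulsing core glow.
; Multi-shot, with barrel glow and UV-offset shot counter, and clip insert/eject sequences are present but unconnected.
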(event OnComponentBeginOverlap(Box)
  (params (OverlappedComponent :type Primitive%20Component%20Object%20Reference) (OtherActor :type Actor%20Object%20Reference) (OtherComp :type Primitive%20Component%20Object%20Reference) (OtherBodyIndex :type Integer) (bFromSweep :type Boolean) (SweepResult :type Hit%20Result%20Structure%20%28by%20ref%29))
  (bind _rifle_core (Variables|Default|GetRifle_Core))
  ;[1 1 1] Single Shot
  (Components|Animation|PlayAnimation (Variables|Default|GetAutomatic_Rifle) "/Game/Automatic_Rifle/Animation/AS_Automatic_Rifle_Shot_Single.AS_Automatic_Rifle_Shot_Single" false)
  (Utilities|FlowControl|Sequence
    (:then_0
      (Audio|Components|Audio|Play (Variables|Default|GetCue_Rifle_Single_Shot_Combined) 0.0)
      (Utilities|FlowControl|Delay 0.13)
      (Rendering|SetVisibility (Variables|Default|GetRifle_Cartrige_Case) false false)
      (Utilities|FlowControl|Delay 0.15)
      (Rendering|SetVisibility (Variables|Default|GetRifle_Cartrige_Case) true false))
    (:then_1
      (Components|Activation|Activate (Variables|Default|GetPS_Rifle_Single_Shot) false)
      (Rendering|Material|SetScalarParameterValueonMaterials _rifle_core "Emissive_Power" 2.0)
      (Utilities|FlowControl|Delay 0.13)
      (Rendering|Material|SetScalarParameterValueonMaterials _rifle_core "Emissive_Power" 0.0))))

(event OnComponentEndOverlap(Box)
  (params (OverlappedComponent :type Primitive%20Component%20Object%20Reference) (OtherActor :type Actor%20Object%20Reference) (OtherComp :type Primitive%20Component%20Object%20Reference) (OtherBodyIndex :type Integer))
  (bind _rifle_core (Variables|Default|GetRifle_Core))
  ;[1 1 1] Single Shot
  (Components|Animation|PlayAnimation (Variables|Default|GetAutomatic_Rifle) "/Game/Automatic_Rifle/Animation/AS_Automatic_Rifle_Shot_Single.AS_Automatic_Rifle_Shot_Single" false)
  (Utilities|FlowControl|Sequence
    (:then_0
      (Audio|Components|Audio|Play (Variables|Default|GetCue_Rifle_Single_Shot_Combined) 0.0)
      (Utilities|FlowControl|Delay 0.13)
      (Rendering|SetVisibility (Variables|Default|GetRifle_Cartrige_Case) false false)
      (Utilities|FlowControl|Delay 0.15)
      (Rendering|SetVisibility (Variables|Default|GetRifle_Cartrige_Case) true false))
    (:then_1
      (Components|Activation|Activate (Variables|Default|GetPS_Rifle_Single_Shot) false)
      (Rendering|Material|SetScalarParameterValueonMaterials _rifle_core "Emissive_Power" 2.0)
      (Utilities|FlowControl|Delay 0.13)
      (Rendering|Material|SetScalarParameterValueonMaterials _rifle_core "Emissive_Power" 0.0))))

(event EventBeginPlay
  (bind _automatic_rifle (Variables|Default|GetAutomatic_Rifle))
  ;[1 1 1] Idle
  (Transformation|AttachComponentToComponent (Variables|Default|GetRifle_Core) _automatic_rifle "CoreSocket" "KeepWorld" "KeepWorld" "KeepWorld" true)
  (Transformation|AttachComponentToComponent (Variables|Default|GetRifle_Cartrige_Case) _automatic_rifle "Cartrige_CaseSocket" "KeepWorld" "KeepWorld" "KeepWorld" true)
  (Transformation|AttachComponentToComponent (Variables|Default|GetRifle_Cartrige_Case) _automatic_rifle "Cartrige_CaseSocket" "KeepWorld" "KeepWorld" "KeepWorld" true)
  (Rendering|Material|SetScalarParameterValueonMaterials (Variables|Default|GetAutomatic_Rifle) "Emissive_Power" 1.0)
  (Rendering|Material|SetScalarParameterValueonMaterials (Variables|Default|GetDigital_Plate_1) "U_Offset" 0.181)
  (Rendering|Material|SetScalarParameterValueonMaterials (Variables|Default|GetDigital_Plate_2) "U_Offset" 0.82))

(fn ConstructionScript)