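; Automatic rifle showcase actor that plays a clip eject when something begins overlapping its Box and a clip insert when the overlap ends.
; Each event pairs an animation and sound cue with timed delays that hide or show the clip bone and digital plates and switch the rifle's emissive.
; The plates act as a digital counter by shifting a U_Offset material parameter.
; Single-shot and multi-shot sequences are present but never run.
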(event OnComponentBeginOverlap(Box)
  (params (OverlappedComponent :type Primitive%20Component%20Object%20Reference) (OtherActor :type Actor%20Object%20Reference) (OtherComp :type Primitive%20Component%20Object%20Reference) (OtherBodyIndex :type Integer) (bFromSweep :type Boolean) (SweepResult :type Hit%20Result%20Structure%20%28by%20ref%29))
  ;[1 1 1] Clip Eject
  (Components|Animation|PlayAnimation (Variables|Default|GetAutomatic_Rifle) "/Game/Automatic_Rifle/Animation/AS_Automatic_Rifle_Clip_Eject.AS_Automatic_Rifle_Clip_Eject" false)
  (Audio|Components|Audio|Play (Variables|Default|GetCue_Rifle_Clip_Eject) 0.0)
  (Rendering|Material|SetScalarParameterValueonMaterials (Variables|Default|GetDigital_Plate_1) "U_Offset" 0.181)
  (Rendering|Material|SetScalarParameterValueonMaterials (Variables|Default|GetDigital_Plate_2) "U_Offset" 0.82)
  (Utilities|FlowControl|Delay 0.5)
  (Rendering|Material|SetScalarParameterValueonMaterials (Variables|Default|GetDigital_Plate_1) "U_Offset" 0.91)
  (Rendering|Material|SetScalarParameterValueonMaterials (Variables|Default|GetAutomatic_Rifle) "Emissive_Power" 0.0)
  (Utilities|FlowControl|Delay 0.1)
  (Rendering|SetVisibility (Variables|Default|GetDigital_Plate_1) false false)
  (Utilities|FlowControl|Delay 0.35)
  (Components|SkinnedMesh|HideBonebyName (Variables|Default|GetAutomatic_Rifle) "Clip" "PBO_None"))

(event OnComponentEndOverlap(Box)
  (params (OverlappedComponent :type Primitive%20Component%20Object%20Reference) (OtherActor :type Actor%20Object%20Reference) (OtherComp :type Primitive%20Component%20Object%20Reference) (OtherBodyIndex :type Integer))
  (bind _digital_plate_1 (Variables|Default|GetDigital_Plate_1))
  ;[1 1 1] Clip Insert
  (Rendering|SetVisibility (Variables|Default|GetDigital_Plate_3) false false)
  (Components|SkinnedMesh|UnHideBonebyName (Variables|Default|GetAutomatic_Rifle) "Clip")
  (Components|Animation|PlayAnimation (Variables|Default|GetAutomatic_Rifle) "/Game/Automatic_Rifle/Animation/AS_Automatic_Rifle_Clip_Insert.AS_Automatic_Rifle_Clip_Insert" false)
  (Rendering|Material|SetScalarParameterValueonMaterials (Variables|Default|GetAutomatic_Rifle) "Emissive_Power" 0.0)
  (Audio|Components|Audio|Play (Variables|Default|GetCue_Rifle_Clip_Insert) 0.0)
  (Utilities|FlowControl|Delay 0.6)
  (Rendering|SetVisibility _digital_plate_1 true false)
  (Rendering|Material|SetScalarParameterValueonMaterials _digital_plate_1 "U_Offset" 0.91)
  (Utilities|FlowControl|Delay 0.1)
  (Rendering|Material|SetScalarParameterValueonMaterials (Variables|Default|GetDigital_Plate_1) "U_Offset" 0.181)
  (Rendering|Material|SetScalarParameterValueonMaterials (Variables|Default|GetDigital_Plate_2) "U_Offset" 0.82)
  (Rendering|Material|SetScalarParameterValueonMaterials (Variables|Default|GetAutomatic_Rifle) "Emissive_Power" 1.0))

(event EventBeginPlay
  (bind _automatic_rifle (Variables|Default|GetAutomatic_Rifle))
  ;[1 1 1] Idle
  (Transformation|AttachComponentToComponent (Variables|Default|GetRifle_Core) _automatic_rifle "CoreSocket" "KeepWorld" "KeepWorld" "KeepWorld" true)
  (Transformation|AttachComponentToComponent (Variables|Default|GetRifle_Cartrige_Case) _automatic_rifle "Cartrige_CaseSocket" "KeepWorld" "KeepWorld" "KeepWorld" true)
  (Transformation|AttachComponentToComponent (Variables|Default|GetRifle_Cartrige_Case) _automatic_rifle "Cartrige_CaseSocket" "KeepWorld" "KeepWorld" "KeepWorld" true)
  (Rendering|Material|SetScalarParameterValueonMaterials (Variables|Default|GetAutomatic_Rifle) "Emissive_Power" 1.0)
  (Rendering|Material|SetScalarParameterValueonMaterials (Variables|Default|GetDigital_Plate_1) "U_Offset" 0.181)
  (Rendering|Material|SetScalarParameterValueonMaterials (Variables|Default|GetDigital_Plate_2) "U_Offset" 0.82))

(fn ConstructionScript)