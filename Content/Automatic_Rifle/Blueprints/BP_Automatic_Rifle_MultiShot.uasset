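; Automatic rifle display actor that plays a scripted multi-shot burst when something overlaps its Box.
; BeginPlay attaches core and cartridge case to sockets; overlap runs animation, sound, particles, core glow and case flicker in parallel Delay chains.
; Delay loops ramp barrel emissive up until a timed flag reverses it, while U_Offset steps animate the digital shot counter.
; Single-shot, clip-insert and clip-eject chains are present but never run.
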(event OnComponentBeginOverlap(Box)
  (params (OverlappedComponent :type Primitive%20Component%20Object%20Reference) (OtherActor :type Actor%20Object%20Reference) (OtherComp :type Primitive%20Component%20Object%20Reference) (OtherBodyIndex :type Integer) (bFromSweep :type Boolean) (SweepResult :type Hit%20Result%20Structure%20%28by%20ref%29))
  (bind _digital_plate_1 (Variables|Default|GetDigital_Plate_1))
  (bind _digital_plate_2 (Variables|Default|GetDigital_Plate_2))
  (bind _rifle_cartrige_case (Variables|Default|GetRifle_Cartrige_Case))
  (bind _rifle_cartrige_case_2 (Variables|Default|GetRifle_Cartrige_Case))
  (bind _rifle_cartrige_case_3 (Variables|Default|GetRifle_Cartrige_Case))
  (bind _rifle_cartrige_case_4 (Variables|Default|GetRifle_Cartrige_Case))
  (bind _rifle_cartrige_case_5 (Variables|Default|GetRifle_Cartrige_Case))
  (bind _rifle_cartrige_case_6 (Variables|Default|GetRifle_Cartrige_Case))
  (bind _rifle_cartrige_case_7 (Variables|Default|GetRifle_Cartrige_Case))
  (bind _rifle_cartrige_case_8 (Variables|Default|GetRifle_Cartrige_Case))
  (bind _rifle_cartrige_case_9 (Variables|Default|GetRifle_Cartrige_Case))
  (bind _rifle_cartrige_case_10 (Variables|Default|GetRifle_Cartrige_Case))
  (bind _rifle_core (Variables|Default|GetRifle_Core))
  ;[1 1 1] Multi Shot
  (Components|Animation|PlayAnimation (Variables|Default|GetAutomatic_Rifle) "/Game/Automatic_Rifle/Animation/AS_Automatic_Rifle_Shot_Multi.AS_Automatic_Rifle_Shot_Multi" false)
  (Utilities|FlowControl|Sequence
    (:then_0
      (Audio|Components|Audio|Play (Variables|Default|GetCue_Rifle_18Shots) 0.0)
      (Utilities|FlowControl|Delay 0.11)
      (Rendering|SetVisibility _rifle_cartrige_case_5 false false)
      (Utilities|FlowControl|Delay 0.057)
      (Rendering|SetVisibility _rifle_cartrige_case_5 true false)
      (Utilities|FlowControl|Delay 0.11)
      (Rendering|SetVisibility _rifle_cartrige_case_6 false false)
      (Utilities|FlowControl|Delay 0.056)
      (Rendering|SetVisibility _rifle_cartrige_case_6 true false)
      (Utilities|FlowControl|Delay 0.11)
      (Rendering|SetVisibility _rifle_cartrige_case_7 false false)
      (Utilities|FlowControl|Delay 0.057)
      (Rendering|SetVisibility _rifle_cartrige_case_7 true false)
      (Utilities|FlowControl|Delay 0.11)
      (Rendering|SetVisibility _rifle_cartrige_case_8 false false)
      (Utilities|FlowControl|Delay 0.056)
      (Rendering|SetVisibility _rifle_cartrige_case_8 true false)
      (Utilities|FlowControl|Delay 0.11)
      (Rendering|SetVisibility _rifle_cartrige_case_3 false false)
      (Utilities|FlowControl|Delay 0.057)
      (Rendering|SetVisibility _rifle_cartrige_case_3 true false)
      (Utilities|FlowControl|Delay 0.11)
      (Rendering|SetVisibility _rifle_cartrige_case_4 false false)
      (Utilities|FlowControl|Delay 0.056)
      (Rendering|SetVisibility _rifle_cartrige_case_4 true false)
      (Utilities|FlowControl|Delay 0.11)
      (Rendering|SetVisibility _rifle_cartrige_case_9 false false)
      (Utilities|FlowControl|Delay 0.057)
      (Rendering|SetVisibility _rifle_cartrige_case_9 true false)
      (Utilities|FlowControl|Delay 0.11)
      (Rendering|SetVisibility _rifle_cartrige_case_10 false false)
      (Utilities|FlowControl|Delay 0.056)
      (Rendering|SetVisibility _rifle_cartrige_case_10 true false)
      (Utilities|FlowControl|Delay 0.11)
      (Rendering|SetVisibility _rifle_cartrige_case_2 false false)
      (Utilities|FlowControl|Delay 0.057)
      (Rendering|SetVisibility _rifle_cartrige_case_2 true false)
      (Utilities|FlowControl|Delay 0.11)
      (Rendering|SetVisibility _rifle_cartrige_case false false)
      (Utilities|FlowControl|Delay 0.056)
      (Rendering|SetVisibility _rifle_cartrige_case true false))
    (:then_1
      (Rendering|Material|SetScalarParameterValueonMaterials _rifle_core "Emissive_Power" 1.0)
      (Utilities|FlowControl|Delay 1.667)
      (Rendering|Material|SetScalarParameterValueonMaterials _rifle_core "Emissive_Power" 0.0))
    (:then_2
      (if (<= 0.0 1.0) :!label _label
        (Utilities|FlowControl|Sequence
          (:then_0
            (Utilities|FlowControl|Delay 0.1)
            (if (<= 0.0 (stale _output_get_2))
              (if (Variables|Default|GetBarrelEmissive_BreakRise)
                (if (<= 0.0 1.0) :!label _label_2
                  (Utilities|FlowControl|Sequence
                    (:then_0
                      (Utilities|FlowControl|Delay 0.1)
                      (if (<= 0.0 (stale _output_get))
                        (bind _output_get (Variables|Default|SetTest (+ (Variables|Default|GetTest) -0.05)))
                        (goto _label_2)))
                    (:then_1
                      (Rendering|Material|SetScalarParameterValueonMaterials (Variables|Default|GetRifle_Barrel) "Emissive_Power" _output_get))))
                (else
                  (bind _output_get_2 (Variables|Default|SetTest (+ (Variables|Default|GetTest) 0.06)))
                  (goto _label)))))
          (:then_1
            (Rendering|Material|SetScalarParameterValueonMaterials (Variables|Default|GetRifle_Barrel) "Emissive_Power" _output_get_2)))))
    (:then_3
      (Components|Activation|Activate (Variables|Default|GetPS_Rifle_Multi_Shot) false)
      (Utilities|FlowControl|Delay 1.66)
      (Variables|Default|SetBarrelEmissive_BreakRise true))
    (:then_4
      ;[1 1 1] Shot Count
      (Rendering|Material|SetScalarParameterValueonMaterials _digital_plate_2 "U_Offset" 0.73)
      (Utilities|FlowControl|Delay 0.09)
      (Rendering|Material|SetScalarParameterValueonMaterials _digital_plate_2 "U_Offset" 0.64)
      (Utilities|FlowControl|Delay 0.09)
      (Rendering|Material|SetScalarParameterValueonMaterials _digital_plate_2 "U_Offset" 0.55)
      (Utilities|FlowControl|Delay 0.09)
      (Rendering|Material|SetScalarParameterValueonMaterials _digital_plate_2 "U_Offset" 0.46)
      (Utilities|FlowControl|Delay 0.09)
      (Rendering|Material|SetScalarParameterValueonMaterials _digital_plate_2 "U_Offset" 0.37)
      (Utilities|FlowControl|Delay 0.09)
      (Rendering|Material|SetScalarParameterValueonMaterials _digital_plate_2 "U_Offset" 0.27)
      (Utilities|FlowControl|Delay 0.09)
      (Rendering|Material|SetScalarParameterValueonMaterials _digital_plate_2 "U_Offset" 0.18)
      (Utilities|FlowControl|Delay 0.09)
      (Rendering|Material|SetScalarParameterValueonMaterials _digital_plate_2 "U_Offset" 0.1)
      (Utilities|FlowControl|Delay 0.09)
      (Rendering|Material|SetScalarParameterValueonMaterials _digital_plate_2 "U_Offset" 0.99)
      (Utilities|FlowControl|Delay 0.09)
      (Rendering|Material|SetScalarParameterValueonMaterials _digital_plate_2 "U_Offset" 0.82)
      (Utilities|FlowControl|Delay 0.09)
      (Rendering|Material|SetScalarParameterValueonMaterials _digital_plate_2 "U_Offset" 0.73)
      (Utilities|FlowControl|Delay 0.09)
      (Rendering|Material|SetScalarParameterValueonMaterials _digital_plate_2 "U_Offset" 0.64)
      (Utilities|FlowControl|Delay 0.09)
      (Rendering|Material|SetScalarParameterValueonMaterials _digital_plate_2 "U_Offset" 0.55)
      (Utilities|FlowControl|Delay 0.09)
      (Rendering|Material|SetScalarParameterValueonMaterials _digital_plate_2 "U_Offset" 0.46)
      (Utilities|FlowControl|Delay 0.09)
      (Rendering|Material|SetScalarParameterValueonMaterials _digital_plate_2 "U_Offset" 0.37)
      (Utilities|FlowControl|Delay 0.09)
      (Rendering|Material|SetScalarParameterValueonMaterials _digital_plate_2 "U_Offset" 0.27)
      (Utilities|FlowControl|Delay 0.09)
      (Rendering|Material|SetScalarParameterValueonMaterials _digital_plate_2 "U_Offset" 0.18)
      (Utilities|FlowControl|Delay 0.09)
      (Rendering|Material|SetScalarParameterValueonMaterials _digital_plate_2 "U_Offset" 0.1)
      (Utilities|FlowControl|Delay 0.09))
    (:then_5
      (Rendering|Material|SetScalarParameterValueonMaterials _digital_plate_1 "U_Offset" 0.1)
      (Utilities|FlowControl|Delay 0.9)
      (Rendering|Material|SetScalarParameterValueonMaterials _digital_plate_1 "U_Offset" 1.0))))

(event EventBeginPlay
  (bind _automatic_rifle (Variables|Default|GetAutomatic_Rifle))
  ;[1 1 1] Idle
  (Transformation|AttachComponentToComponent (Variables|Default|GetRifle_Core) _automatic_rifle "CoreSocket" "KeepWorld" "KeepWorld" "KeepWorld" true)
  (Transformation|AttachComponentToComponent (Variables|Default|GetRifle_Cartrige_Case) _automatic_rifle "Cartrige_CaseSocket" "KeepWorld" "KeepWorld" "KeepWorld" true)
  (Transformation|AttachComponentToComponent (Variables|Default|GetRifle_Cartrige_Case) _automatic_rifle "Cartrige_CaseSocket" "KeepWorld" "KeepWorld" "KeepWorld" true)
  (Rendering|Material|SetScalarParameterValueonMaterials (Variables|Default|GetAutomatic_Rifle) "Emissive_Power" 1.0)
  (Rendering|Material|SetScalarParameterValueonMaterials (Variables|Default|GetDigital_Plate_1) "U_Offset" 0.181)
  (Rendering|Material|SetScalarParameterValueonMaterials (Variables|Default|GetDigital_Plate_2) "U_Offset" 0.82))

(fn ConstructionScript)