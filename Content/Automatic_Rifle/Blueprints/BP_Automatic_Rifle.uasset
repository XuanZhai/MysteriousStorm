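; Automatic rifle actor that presents weapon animations, sounds and effects, with no projectile or damage logic.
; BeginPlay attaches the core and cartridge case to sockets and sets the initial glow and digital counter.
; Unwired chains for single shot, multi shot, clip insert and clip eject time case visibility, emissive changes and clip-bone hiding with Delays.
; The counter scrolls material U offsets; barrel heat glow ramps through a delayed loop.
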(event OnComponentBeginOverlap(Box)
  (params (OverlappedComponent :type Primitive%20Component%20Object%20Reference) (OtherActor :type Actor%20Object%20Reference) (OtherComp :type Primitive%20Component%20Object%20Reference) (OtherBodyIndex :type Integer) (bFromSweep :type Boolean) (SweepResult :type Hit%20Result%20Structure%20%28by%20ref%29)))

(event EventBeginPlay
  (bind _automatic_rifle (Variables|Default|GetAutomatic_Rifle))
  ;[1 1 1] Idle
  (Transformation|AttachComponentToComponent (Variables|Default|GetRifle_Core) _automatic_rifle "CoreSocket" "KeepWorld" "KeepWorld" "KeepWorld" true)
  (Transformation|AttachComponentToComponent (Variables|Default|GetRifle_Cartrige_Case) _automatic_rifle "Cartrige_CaseSocket" "KeepWorld" "KeepWorld" "KeepWorld" true)
  (Transformation|AttachComponentToComponent (Variables|Default|GetRifle_Cartrige_Case) _automatic_rifle "Cartrige_CaseSocket" "KeepWorld" "KeepWorld" "KeepWorld" true)
  (Rendering|Material|SetScalarParameterValueonMaterials (Variables|Default|GetAutomatic_Rifle) "Emissive_Power" 1.0)
  (Rendering|Material|SetScalarParameterValueonMaterials (Variables|Default|GetDigital_Plate_1) "U_Offset" 0.181)
  (Rendering|Material|SetScalarParameterValueonMaterials (Variables|Default|GetDigital_Plate_2) "U_Offset" 0.82))

(fn ConstructionScript)