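; BP_Hit is a short-lived shield impact effect actor, set up through its OnHit event.
; OnHit copies the passed mesh's static mesh, applies a hit material as a dynamic instance and sets its color.
; A timeline then drives hit position (offset from the mesh's location), size-scaled radius (parameter spelled "Raidus") and opacity.
; The actor destroys itself when the timeline finishes.
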(event EventBeginPlay)

(event Collision|EventActorBeginOverlap
  (params (OtherActor :type Actor%20Object%20Reference)))

(event EventOnHit
  (params (HitLocation :type Vector :default "0, 0, 0") (Mesh :type Static%20Mesh%20Component%20Object%20Reference) (HitMaterial :type Material%20Interface%20Object%20Reference) (HitSize :type Float%20%28single-precision%29) (HitColor :type Linear%20Color%20Structure))
  (bind _staticmesh (Variables|Default|GetStaticMesh))
  (Utilities|IsValid Mesh
    (:Is%20Valid
      (Components|StaticMesh|SetStaticMesh (Variables|/Script/Engine.StaticMeshComponent|GetStaticMesh Mesh))
      (Rendering|Material|SetMaterial _staticmesh 0 HitMaterial)
      (Utilities|FlowControl|Sequence
        (:then_0
          (bind _returnvalue (Rendering|Material|CreateDynamicMaterialInstance _staticmesh 0 HitMaterial "None" :!class /Script/Engine.PrimitiveComponent))
          (Variables|Default|SetHitSize HitSize)
          (Rendering|Material|SetVectorParameterValue _returnvalue "Color" HitColor :!class /Script/Engine.MaterialInstanceDynamic))
        (:then_1
          (bind (_direction _opacity _hitsize) (Timeline|Timeline_0 PlayFromStart)
            (:Update
              (Rendering|Material|SetVectorParameterValue _returnvalue "HitPosition" (Math|Conversions|ToLinearColor(Vector) (+ HitLocation (Transformation|GetWorldLocation Mesh))) :!class /Script/Engine.MaterialInstanceDynamic)
              (Rendering|Material|SetScalarParameterValue _returnvalue "Raidus" (* _hitsize (Variables|Default|GetHitSize)) :!class /Script/Engine.MaterialInstanceDynamic)
              (Rendering|Material|SetScalarParameterValue _returnvalue "Opacity" _opacity :!class /Script/Engine.MaterialInstanceDynamic))
            (:Finished
              (Actor|DestroyActor))))))))

(event EventTick
  (params (DeltaSeconds :type Float%20%28single-precision%29)))

(fn ConstructionScript)

(fn GetShieldRef
  (return 0))