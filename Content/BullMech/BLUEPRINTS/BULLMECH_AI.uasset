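; AI controller for the BullMech enemy, which runs its behavior tree on BeginPlay and stores the possessed character.
; AI perception updates write the CanSeePlayer blackboard key whenever the player character is sensed or lost.
; While the IsChasing key is set, Tick sphere-traces ahead and slightly downward and makes the pawn jump on a hit, a demo-only workaround for blocking walls.
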(event OnTargetPerceptionUpdated(AIPerception)
  (params (Actor :type Actor%20Object%20Reference) (Stimulus :type AI%20Stimulus%20Structure))
  ;[1 1 1] Can See Player? Then look at Behaviour Tree
  (Utilities|Casting|CastToThirdPersonCharacter Actor)
  (AI|Components|Blackboard|SetValueasBool (AI|GetBlackboard 0) (Utilities|Name|MakeLiteralName "CanSeePlayer") (.bSuccessfullySensed (Utilities|Struct|BreakAIStimulus Stimulus))))

(event EventBeginPlay
  (AI|RunBehaviorTree "/Game/BullMech/BLUEPRINTS/BULLMECH_BT.BULLMECH_BT"))

(event EventTick
  (params (DeltaSeconds :type Float%20%28single-precision%29))
  (bind _storepawn (Variables|Default|GetStorePawn))
  (bind _returnvalue (Transformation|GetActorLocation _storepawn))
  (bind _returnvalue_2 (Transformation|GetActorForwardVector _storepawn))
  (bind _returnvalue_3 (* _returnvalue_2 2.5e+02))
  (bind (_x _y _z) (Math|Vector|BreakVector _returnvalue_3))
  ;[1 1 1] Jump stimulus. A bit hacky. If chasing and be blocked by a wall, then Jump. Only for demonstrational purposes
  (if (ScalableFloat|GetValueasBool (AI|GetBlackboard 0) (Utilities|Name|MakeLiteralName "IsChasing"))
    (bind _returnvalue_4 (Collision|SphereTraceByChannel _returnvalue (+ _returnvalue (Math|Vector|MakeVector _x _y (- _z 7e+01))) 2e+01 "TraceTypeQuery1" false 0 "None"))
    (if _returnvalue_4
      (Character|Jump (Variables|Default|GetStorePawn)))))

(event EventOnPossess
  (params (PossessedPawn :type Pawn%20Object%20Reference))
  (bind _ascharacter (Utilities|Casting|CastToCharacter PossessedPawn))
  (Variables|Default|SetStorePawn _ascharacter))

(fn ConstructionScript)