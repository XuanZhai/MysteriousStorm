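; Placeable dust and sandstorm volume that fills a configurable Tile grid with Niagara components spaced by Area.
; The Construction Script adds the components, steps them through X, Y and Z by array index, centers them horizontally and fits a box to the volume.
; It then pushes exposed dust, particle and particle-line settings into each component.
; The Event Graph holds only an unconnected template for changing parameters at runtime.
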(event EventBeginPlay)

(event Collision|EventActorBeginOverlap
  (params (OtherActor :type Actor%20Object%20Reference)))

(event EventTick
  (params (DeltaSeconds :type Float%20%28single-precision%29)))

(fn ConstructionScript
  (bind _box (Variables|Default|GetBox))
  (bind _tile (Variables|Default|GetTile))
  (bind _area (Variables|Basic|GetArea))
  (bind _tile_2 (Variables|Default|GetTile))
  (bind _tile_3 (Variables|Default|GetTile))
  (bind _area_2 (Variables|Basic|GetArea))
  (bind _tile_4 (Variables|Default|GetTile))
  (bind (_x _y _z) (Math|Vector|BreakVector _tile_2))
  (bind (_x_2 _y_2) (Math|Vector|BreakVector _tile_3))
  (bind (_x_3 _y_3 _z_2) (Math|Vector|BreakVector _tile_4))
  (bind (_x_4 _y_4 _z_3) (Math|Vector|BreakVector _tile))
  (bind _returnvalue (* _area_2 0.5))
  (bind _returnvalue_2 (Math|Float|Absolute(Float) _x_2))
  (bind _returnvalue_3 (* _z_2 _returnvalue))
  (bind _returnvalue_4 (Math|Float|Truncate _returnvalue_2))
  ;[0 0.8793 1 1 100] Add Niagara Component
  (for _index (range 1 (Math|Float|Truncate (* (Math|Float|Absolute(Float) _x) (Math|Float|Absolute(Float) _y) (Math|Float|Absolute(Float) _z))))
    (bind _returnvalue_5 (AddComponent|AddNiagaraComponent false (Math|Transform|MakeTransform "0, 0, 0")))
    (Utilities|Array|SetArrayElem (Variables|Default|GetNiagara) _index _returnvalue_5 true))
  ;[0 0.09986 1 1 100] Set Niagara Location
  (for (_array_element _array_index) (Variables|Default|GetNiagara)
    (Transformation|AddRelativeLocation _array_element (Math|Vector|MakeVector (* (Math|Integer|%(Integer) _array_index _returnvalue_4) (Variables|Basic|GetArea)) (* (Variables|Default|Getplus) (Variables|Basic|GetArea)) (* (Variables|Default|Getplus_z) (Variables|Basic|GetArea))) false false)
    (if (and (== (Math|Integer|%(Integer) _array_index _returnvalue_4) 0) (> _array_index 0))
      (bind _result (Math|Integer|IncrementInt (Variables|Default|Getplus))
        (:%20%20
          (Variables|Default|Setplus _result)
          (if (== (Math|Integer|%(Integer) _array_index (* _returnvalue_4 (Math|Float|Truncate (Math|Float|Absolute(Float) _y_2)))) 0)
            (Variables|Default|Setplus 0)
            (bind _result_2 (Math|Integer|IncrementInt (Variables|Default|Getplus_z))
              (:%20%20
                (Variables|Default|Setplus_z _result_2))))))))
  ;[0.8222 1 0.07767 1 100] Offset Niagara Location
  (for _array_element_2 (Variables|Default|GetNiagara)
    (Transformation|AddRelativeLocation _array_element_2 (Math|Vector|MakeVector (* (* (- (Math|Float|Truncate (Math|Float|Absolute(Float) _x_4)) 1) _area) -0.5) (* (* (- (Math|Float|Truncate (Math|Float|Absolute(Float) _y_4)) 1) _area) -0.5) (* _area 0.5)) false false))
  ;[0.3789 0 1 1 100] Set Size and Box Collision Location
  (Components|Box|SetBoxExtent _box (Math|Vector|MakeVector (* _x_3 _returnvalue) (* _y_3 _returnvalue) _returnvalue_3) true)
  (Transformation|SetRelativeLocation _box (Math|Vector|MakeVector 0.0 0.0 _returnvalue_3) false false)
  ;[1 0 0.8974 1 100] Set Niagara Parameters
  (for _array_element_3 (Variables|Default|GetNiagara)
    (Variables|Default|SetDust _array_element_3)
    (Niagara|SetNiagaraVariable(Float) (Variables|Default|GetDust) "Area" (Variables|Basic|GetArea))
    (Niagara|SetNiagaraVariable(Float) (Variables|Default|GetDust) "Noise Frequency" (Variables|Basic|GetNoise%20Frequency))
    (Niagara|SetNiagaraVariable(Float) (Variables|Default|GetDust) "Noise Strength" (Variables|Basic|GetNoise%20Strength))
    (Niagara|SetNiagaraVariable(Float) (Variables|Default|GetDust) "LifeTime_Scale" (Variables|Basic|GetLifeTime_Scale))
    (Niagara|SetNiagaraVariable(Float) (Variables|Default|GetDust) "VelocityToCamera" (Variables|Basic|GetVelocityToCamera))
    (Niagara|SetNiagaraVariable(Float) (Variables|Default|GetDust) "Velocity Speed Scale" (Variables|Basic|GetVelocity))
    (Niagara|SetNiagaraVariable(Float) (Variables|Default|GetDust) "DustContrast" (Variables|Smoke|GetDustContrast))
    (Niagara|SetNiagaraVariable(Float) (Variables|Default|GetDust) "DustSize_Scale" (Variables|Smoke|GetDustSize_Scale))
    (Niagara|SetNiagaraVariable(Float) (Variables|Default|GetDust) "Emessive_Dust" (Variables|Smoke|GetEmessive_Dust))
    (Niagara|SetNiagaraVariable(Float) (Variables|Default|GetDust) "SpawnRate_Dust" (Variables|Smoke|GetSpawnRate_Dust))
    (Niagara|SetNiagaraVariable(LinearColor) (Variables|Default|GetDust) "TintDust" (Variables|Smoke|GetTintDust))
    (Niagara|SetNiagaraVariable(Float) (Variables|Default|GetDust) "Emessive_Particle" (Variables|Particle|GetEmessive_Particle))
    (Niagara|SetNiagaraVariable(Float) (Variables|Default|GetDust) "ParticleContrast" (Variables|Particle|GetParticleContrast))
    (Niagara|SetNiagaraVariable(Float) (Variables|Default|GetDust) "Size_particle" (Variables|Particle|GetParticleSize_Scale))
    (Niagara|SetNiagaraVariable(Float) (Variables|Default|GetDust) "SpawnRate_particle" (Variables|Particle|GetSpawnRate_Particle))
    (Niagara|SetNiagaraVariable(LinearColor) (Variables|Default|GetDust) "TintParticleColor" (Variables|Particle|GetTintParticle))
    (Niagara|SetNiagaraVariable(Float) (Variables|Default|GetDust) "Emessive_particleLine" (Variables|Particle_Line|GetEmessive_Particle_Line))
    (Niagara|SetNiagaraVariable(Float) (Variables|Default|GetDust) "ParticleLineContrast" (Variables|Particle_Line|GetParticleContrast_Line))
    (Niagara|SetNiagaraVariable(Float) (Variables|Default|GetDust) "Size_ParticleLine" (Variables|Particle_Line|GetParticleSize_Scale_Line))
    (Niagara|SetNiagaraVariable(Float) (Variables|Default|GetDust) "SpawnRate_particleLine" (Variables|Particle_Line|GetSpawnRate_Particle_Line))
    (Niagara|SetNiagaraVariable(LinearColor) (Variables|Default|GetDust) "TintParticleLine" (Variables|Particle_Line|GetTintParticle_Line))))