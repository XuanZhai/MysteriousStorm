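; BP_SplineDust is a spline-driven sandstorm dust actor that exposes tuning for a Niagara effect.
; Its construction script passes the Spline component and noise, smoke, particle, color, emissive and contrast settings to the SplineDust Niagara component.
; ColorMinimum and ColorMaximum both write to "Color Minimum", so the maximum value overwrites the minimum.
; The event graph holds only disabled placeholder events, so the Blueprint adds no runtime logic.
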(event EventBeginPlay)

(event Collision|EventActorBeginOverlap
  (params (OtherActor :type Actor%20Object%20Reference)))

(event EventTick
  (params (DeltaSeconds :type Float%20%28single-precision%29)))

(fn ConstructionScript
  (bind _splinedust (Variables|Default|GetSplineDust))
  ;[0.6784 0 1 1 100] Set Niagara Parameters
  (Class|NiagaraComponent|SetVariableObject _splinedust "Spline" (Variables|Default|GetSpline))
  (Niagara|SetNiagaraVariable(Float) _splinedust "SandNoise" (Variables|Smoke|GetSandNoise))
  (Niagara|SetNiagaraVariable(Float) _splinedust "SandNoiseScale" (Variables|Smoke|GetSandNoiseScale))
  (Niagara|SetNiagaraVariable(Float) _splinedust "Smoke_SpawnRate" (Variables|Smoke|GetSmoke_SpawnRate))
  (Niagara|SetNiagaraVariable(LinearColor) _splinedust "Color Minimum" (Variables|Basic|GetColor%20Minimum))
  (Niagara|SetNiagaraVariable(LinearColor) _splinedust "Color Minimum" (Variables|Basic|GetColor%20Maximum))
  (Niagara|SetNiagaraVariable(Float) _splinedust "Emessive" (Variables|Basic|GetEmessive))
  (Niagara|SetNiagaraVariable(Float) _splinedust "Contrast" (Variables|Basic|GetContrast))
  (Niagara|SetNiagaraVariable(Float) _splinedust "Particle_SpawnRate" (Variables|Particle|GetParticle_SpawnRate))
  (Niagara|SetNiagaraVariable(Float) _splinedust "SmokeSizeScale" (Variables|Smoke|GetSmokeSizeScale))
  (Niagara|SetNiagaraVariable(Float) _splinedust "ParticleSizeScale" (Variables|Particle|GetParticleSizeScale))
  (Niagara|SetNiagaraVariable(Float) _splinedust "particleAlpha" (Variables|Particle|GetparticleAlpha)))