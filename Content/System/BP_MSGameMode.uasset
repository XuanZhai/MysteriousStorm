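; BP_MSGameMode is a game mode Blueprint that controls the spawning and cleanup of spawner-driven items.
; On BeginPlay it binds handlers to the spawn-items and remove-spawn-items events.
; The spawn handler updates the plan of every BP_ActorSpawner tagged "ControlledByGM", then has it spawn its items.
; The removal handler destroys every actor tagged "FromSpawner", so both sides find their targets by tag instead of stored references.
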(event Custom|OnUpdateItemSpawner
  (bind _outactors (Actor|GetAllActorsOfClasswithTag "/Game/Item/BP_ActorSpawner.BP_ActorSpawner_C" "ControlledByGM"))
  (for _array_element _outactors
    (Class|MSItemSpawner|UpdateSpawnPlan _array_element)
    (Class|MSItemSpawner|SpawnItems _array_element)))

(event Custom|OnRemoveSpawnItems
  (bind _outactors (Actor|GetAllActorsOfClasswithTag "/Script/Engine.Actor" "FromSpawner"))
  (for _array_element _outactors
    (Actor|DestroyActor _array_element)))

(event EventBeginPlay
  (EventDispatchers|BindEventtoSpawnItems (delegate Custom|OnUpdateItemSpawner))
  (EventDispatchers|BindEventtoRemoveSpawnItems (delegate Custom|OnRemoveSpawnItems)))

(event EventTick
  (params (DeltaSeconds :type Float%20%28single-precision%29)))

(fn ConstructionScript
  (|CallParentFunction))