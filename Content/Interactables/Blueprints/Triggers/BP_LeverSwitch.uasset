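; BP_LeverSwitch is a lever switch interactable that animates its lever when its sender trigger fires.
; OnSenderTriggered plays the MoveController timeline, whose RotateDegree track drives the relative roll of the Controller component while keeping its pitch and yaw.
; The timeline only plays forward, with no reverse path, and the Blueprint has no other active logic of its own.
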(event EventBeginPlay
  (|CallParentFunction) ; This node is disabled and will not be called.\nDrag off pins to build functionality.
)

(event Collision|EventActorBeginOverlap
  (params (OtherActor :type Actor%20Object%20Reference))
  (|CallParentFunction OtherActor) ; This node is disabled and will not be called.\nDrag off pins to build functionality.
)

(event EventTick
  (params (DeltaSeconds :type Float%20%28single-precision%29))
  (|CallParentFunction DeltaSeconds) ; This node is disabled and will not be called.\nDrag off pins to build functionality.
)

(event EventOnSenderTriggered
  (bind _controller (Variables|Default|GetController))
  (bind _relativerotation (Variables|/Script/Engine.SceneComponent|GetRelativeRotation _controller))
  ;[1 1 1] Play Animation
  (bind _rotatedegree (Timeline|MoveController Play)
    (:Update
      (Transformation|SetRelativeRotation _controller (Math|Rotator|MakeRotator _rotatedegree (.pitch _relativerotation) (.yaw _relativerotation)) false false))))

(fn ConstructionScript
  (|CallParentFunction))